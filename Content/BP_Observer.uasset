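; BP_Observer is an observer actor that creates the WBP_UI widget on play, shows the mouse cursor, and passes itself to the widget.
; Its To3D and To2D events play one timeline forward or in reverse to blend between a default and a 3D view.
; The timeline interpolates camera rotation, actor location and orthographic width, so the camera zooms in while changing angle.
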(event `self.ReceiveBeginPlay`
  (bind _returnvalue (`|CreateWidget` "/Game/WBP_UI.WBP_UI_C"))
  (`UserWidget.AddToViewport` _returnvalue 0)
  (set `PlayerController.bShowMouseCursor` true (`GameplayStatics.GetPlayerController` 0))
  (set `/Game/WBP_UI.Player` self _returnvalue))

(event `To3D`
  (bind (_direction _newtrack_0) (`Timeline|Anim` :!via `PlayFromStart` :!label _label)
    (:`Update`
      (`SceneComponent.K2_SetWorldRotation` (`self.Camera`) (`KismetMathLibrary.RLerp` (`self.DefCam`) (`self.3D Cam`) _newtrack_0 true) false false)
      (`self.K2_SetActorLocation` (`KismetMathLibrary.VLerp` (`self.DefCamPos`) (`self.3D`) _newtrack_0))
      (`CameraComponent.SetOrthoWidth` (`self.Camera`) (`KismetMathLibrary.Lerp` 25.0 5.0 _newtrack_0)))))

(event `To2D`
  (goto _label :!via `ReverseFromEnd`))

(fn `UserConstructionScript`)